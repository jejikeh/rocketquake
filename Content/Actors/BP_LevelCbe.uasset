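; BP_LevelCbe is a cube actor that gives itself a random scale and moves clear of player starts.
; On its first authority-side tick, it sets its scale to a random unit vector times a random integer below 50, so axes differ and can be negative.
; When its Box component begins overlapping a BP_PlayerStart, the actor jumps 1000 units up without sweeping.
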(event `self.ReceiveTick`
  (params (DeltaSeconds :type "Float (single-precision)"))
  (`/Engine/EditorBlueprintResources/ActorMacros.Switch Has Authority`
    (:`Authority`
      (if (`self.isFirstTick`)
        (set `self.isFirstTick` false)
        (`self.SetActorScale3D` (* (`KismetMathLibrary.RandomUnitVector`) (`KismetMathLibrary.RandomInteger` 50)))))))

(event `self.Cube.OnComponentBeginOverlap`
  (params (OverlappedComponent :type "PrimitiveComponent Object Reference") (OtherActor :type "Actor Object Reference") (OtherComp :type "PrimitiveComponent Object Reference") (OtherBodyIndex :type Integer) (bFromSweep :type Boolean) (SweepResult :type "HitResult Structure (by ref)")))

(event `self.Box.OnComponentBeginOverlap`
  (params (OverlappedComponent :type "PrimitiveComponent Object Reference") (OtherActor :type "Actor Object Reference") (OtherComp :type "PrimitiveComponent Object Reference") (OtherBodyIndex :type Integer) (bFromSweep :type Boolean) (SweepResult :type "HitResult Structure (by ref)"))
  (cast `/Game/BP_PlayerStart` OtherActor)
  (`self.K2_SetActorLocation` (+ (`self.K2_GetActorLocation`) (0.0 0.0 1000.0))))

(fn `UserConstructionScript`)