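; BP_RandomPickup is a placement actor that spawns random health, rifle ammo or launcher ammo pickups, or a randomized point light.
; On authority Tick, it nudges itself upward until a small sphere overlap is clear, then spawns once at that position on a following tick.
; SpawnRandomPickup rolls separately for each of the four options, so one call can spawn none or several.
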(event `self.ReceiveBeginPlay`)

(event `self.ReceiveTick`
  (params (DeltaSeconds :type "Float (single-precision)"))
  (`/Engine/EditorBlueprintResources/ActorMacros.Switch Has Authority`
    (:`Authority`
      (if (`self.bWasSpawned`)
        _
        (elif (`self.bIsFree`)
          (`self.SpawnRandomPickup`)
          (set `self.bWasSpawned` true)
          (else
            (bind (_outactors _returnvalue) (`KismetSystemLibrary.SphereOverlapActors` (`self.K2_GetActorLocation`) 10.0 (`self.Object Types`)))
            (if _returnvalue
              (`self.K2_SetActorLocation` (+ (`self.K2_GetActorLocation`) (0.0 0.0 10.0)))
              (else
                (set `self.bIsFree` true)))))))))

(fn `SpawnRandomPickup`
  (bind _returnvalue (`KismetMathLibrary.RandomIntegerInRange` 0 3))
  (bind _returnvalue_2 (`self.GetTransform`))
  (bind _returnvalue_3 (`KismetMathLibrary.RandomFloatInRange` 100.0 1000.0))
  (`|ExecutionSequence`
    (:`then_0`
      (if (== _returnvalue 0)
        (`|SpawnActorFromClass` "/Game/Actors/BP_HealthPickup.BP_HealthPickup_C" _returnvalue_2 "Undefined" "MultiplyWithRoot" null null)))
    (:`then_1`
      (if (== _returnvalue 1)
        (`|SpawnActorFromClass` "/Game/Actors/BP_RiffleAmmoPickup.BP_RiffleAmmoPickup_C" _returnvalue_2 "Undefined" "MultiplyWithRoot" null null)))
    (:`then_2`
      (if (== _returnvalue 2)
        (`|SpawnActorFromClass` "/Game/Actors/BP_LauncherAmmoPickup.BP_LauncherAmmoPickup_C" _returnvalue_2 "Undefined" "MultiplyWithRoot" null null)))
    (:`then_3`
      (if (== _returnvalue 3)
        (bind _returnvalue_4 (`|SpawnActorFromClass` "/Script/Engine.PointLight" _returnvalue_2 "Undefined" "MultiplyWithRoot" null null))
        (bind _pointlightcomponent (`PointLight.PointLightComponent` _returnvalue_4))
        (`LightComponent.SetIntensity` _pointlightcomponent _returnvalue_3)
        (`LocalLightComponent.SetAttenuationRadius` _pointlightcomponent _returnvalue_3)))))

(fn `UserConstructionScript`)