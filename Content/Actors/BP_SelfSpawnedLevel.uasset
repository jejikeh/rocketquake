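; BP_SelfSpawnedLevel is a self-replicating level chunk that procedurally extends the world as a BP_MainMen moves through it.
; On its first authority Tick, it scatters random counts of BP_LevelCbe and BP_RandomPickup actors in random directions around itself.
; When a BP_MainMen first overlaps its Box, the server spawns the next BP_SelfSpawnedLevel at a fixed X offset, guarded by a flag to spawn only once.
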(event `self.ReceiveTick`
  (params (DeltaSeconds :type "Float (single-precision)"))
  (`/Engine/EditorBlueprintResources/ActorMacros.Switch Has Authority`
    (:`Authority`
      (if (`self.bIsFirstTick`)
        (set `self.bIsFirstTick` false)
        (for _ (range (+ (`KismetMathLibrary.RandomIntegerInRange` 15 30) 1))
          (`|SpawnActorFromClass` "/Game/Actors/BP_LevelCbe.BP_LevelCbe_C" (`KismetMathLibrary.MakeTransform` (+ (`self.K2_GetActorLocation`) (* (`KismetMathLibrary.RandomUnitVector`) (`KismetMathLibrary.RandomIntegerInRange` 1000 4000))) (`self.K2_GetActorRotation`)) "Undefined" "MultiplyWithRoot" null null))
        (for _ (range (+ (`KismetMathLibrary.RandomIntegerInRange` 30 60) 1))
          (`|SpawnActorFromClass` "/Game/Actors/BP_RandomPickup.BP_RandomPickup_C" (`KismetMathLibrary.MakeTransform` (+ (`self.K2_GetActorLocation`) (* (`KismetMathLibrary.RandomUnitVector`) (`KismetMathLibrary.RandomIntegerInRange` 1000 4000)))) "Undefined" "MultiplyWithRoot" null null))))))

(event `self.Box.OnComponentBeginOverlap`
  (params (OverlappedComponent :type "PrimitiveComponent Object Reference") (OtherActor :type "Actor Object Reference") (OtherComp :type "PrimitiveComponent Object Reference") (OtherBodyIndex :type Integer) (bFromSweep :type Boolean) (SweepResult :type "HitResult Structure (by ref)"))
  (bind (_returnvalue_location _returnvalue_rotation _returnvalue_scale) (`KismetMathLibrary.BreakTransform` (`self.GetTransform` self)))
  (`/Engine/EditorBlueprintResources/ActorMacros.Switch Has Authority`
    (:`Authority`
      (if (not (`self.bIsAlreadySpawned`))
        (cast `/Game/Player/BP_MainMen` OtherActor)
        (`|SpawnActorFromClass` "BP_SelfSpawnedLevel_C" (`KismetMathLibrary.MakeTransform` (+ _returnvalue_location (5000.0 0.0 0.0)) _returnvalue_rotation _returnvalue_scale) "Undefined" "MultiplyWithRoot" null null)
        (set `self.bIsAlreadySpawned` true)))))

(fn `UserConstructionScript`)