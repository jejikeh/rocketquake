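; Game Instance that manages multiplayer session hosting and invite joining through Advanced Sessions nodes.
; CreateMatch creates an online session, reported as Steam, and opens L_Menu as a listen server.
; On failure it retries as a LAN session, and if that also fails it opens L_Menu without the listen option.
; An accepted invite destroys the current session and, once that succeeds, joins the invited one.
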(event `CreateMatch`
  (`CreateSessionCallbackProxyAdvanced.CreateAdvancedSession` :`PlayerController` (`GameplayStatics.GetPlayerController` 0)
    (:`OnSuccess`
      (`GameplayStatics.OpenLevelBySoftObjectPtr` "/Game/Menu/L_Menu.L_Menu" true "listen"))
    (:`OnFailure`
      (`KismetSystemLibrary.PrintString` "Failed to create Steam Session, fallback to LAN")
      (`CreateSessionCallbackProxyAdvanced.CreateAdvancedSession` :`PlayerController` (`GameplayStatics.GetPlayerController` 0) :`bUseLAN` true
        (:`OnSuccess`
          (`GameplayStatics.OpenLevelBySoftObjectPtr` "/Game/Menu/L_Menu.L_Menu" true "listen"))
        (:`OnFailure`
          (`KismetSystemLibrary.PrintString` "Failed to create LAN Session")
          (`GameplayStatics.OpenLevelBySoftObjectPtr` "/Game/Menu/L_Menu.L_Menu"))))))

(event `self.OnSessionInviteAccepted`
  (params (LocalPlayerNum :type Integer) (PersonInvited :type "BPUniqueNetId Structure") (SessionToJoin :type "BlueprintSessionResult Structure (by ref)"))
  (`DestroySessionCallbackProxy.DestroySession` (`GameplayStatics.GetPlayerController` 0)
    (:`OnSuccess`
      (`JoinSessionCallbackProxy.JoinSession` (`GameplayStatics.GetPlayerController` 0) SessionToJoin))))