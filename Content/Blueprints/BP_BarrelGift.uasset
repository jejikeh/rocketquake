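; BP_BarrelGift is a destructible barrel that explodes on death and drops a random pickup: health, rifle ammo or launcher ammo.
; The server binds to the HealthComponent's OnDeath, multicasts the explosion effect and sound, spawns the pickup, then destroys the actor.
; Any damage taken also spawns a BP_DamagePoints actor carrying the damage amount.
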(event `Multicast_SpawnVfx`
  (`NiagaraFunctionLibrary.SpawnSystemAtLocation` "/Game/Effects/Particles/Explosion/NS_Grenade_Explosion.NS_Grenade_Explosion" (`self.K2_GetActorLocation`))
  (`GameplayStatics.PlaySoundAtLocation` "/Game/Sounds/Impacts/SCue_Impt_Launcher.SCue_Impt_Launcher" (`self.K2_GetActorLocation`) (struct) 1.0 1.0 0.0 null null null null))

(event `self.ReceiveBeginPlay`
  (`/Engine/EditorBlueprintResources/ActorMacros.Switch Has Authority`
    (:`Authority`
      (add `HealthComponent.OnDeath` (`self.HealthComponent`) (delegate `OnDeath_Event`)))))

(event `OnDeath_Event`
  (bind _returnvalue (`self.GetTransform`))
  (`|ExecutionSequence`
    (:`then_0`
      (`/Engine/EditorBlueprintResources/ActorMacros.Switch Has Authority`
        (:`Authority`
          (`self.Multicast_SpawnVfx`))))
    (:`then_1`
      (switch `int` (`KismetMathLibrary.RandomIntegerInRange` 0 2)
        (:`0`
          (`|SpawnActorFromClass` "/Game/Actors/BP_HealthPickup.BP_HealthPickup_C" _returnvalue "Undefined" "MultiplyWithRoot" null null))
        (:`1`
          (`|SpawnActorFromClass` "/Game/Actors/BP_RiffleAmmoPickup.BP_RiffleAmmoPickup_C" _returnvalue "Undefined" "MultiplyWithRoot" null null))
        (:`2`
          (`|SpawnActorFromClass` "/Game/Actors/BP_LauncherAmmoPickup.BP_LauncherAmmoPickup_C" _returnvalue "Undefined" "MultiplyWithRoot" null null))))
    (:`then_2`
      (`self.K2_DestroyActor`))))

(event `self.ReceiveAnyDamage`
  (params (Damage :type "Float (single-precision)") (DamageType :type "DamageType Object Reference") (InstigatedBy :type "Controller Object Reference") (DamageCauser :type "Actor Object Reference"))
  (`|SpawnActorFromClass` "/Game/Blueprints/BP_DamagePoints.BP_DamagePoints_C" (`self.GetTransform`) "Undefined" "MultiplyWithRoot" null Damage null))

(fn `UserConstructionScript`)