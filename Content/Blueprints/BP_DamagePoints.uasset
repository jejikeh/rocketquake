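; BP_DamagePoints is a floating damage number actor that shows a damage value and drifts away before removing itself.
; On BeginPlay it passes Damage to its WBP_DamagePoints widget and randomizes both start position and travel offset, with the Z minimum taken from negated Offset.Y.
; The MoveT timeline lerps the actor from start to end, then destroys it on finish.
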(event `self.ReceiveBeginPlay`
  (bind (_offset_x _offset_y _offset_z) (`KismetMathLibrary.BreakVector` (`self.Offset`)))
  (set `self.Offset` (`KismetMathLibrary.MakeVector` (`KismetMathLibrary.RandomFloatInRange` (* _offset_x -1.0) _offset_x) (`KismetMathLibrary.RandomFloatInRange` (* _offset_y -1.0) _offset_y) (`KismetMathLibrary.RandomFloatInRange` (* _offset_y -1.0) _offset_z)))
  (bind _aswbp_damage_points (cast `/Game/UI/WBP_DamagePoints` (`WidgetComponent.GetWidget` (`self.Widget`))))
  (set `/Game/UI/WBP_DamagePoints.Damage` (`self.Damage`) _aswbp_damage_points)
  (bind _output_get (set `self.StartLocation` (+ (`self.K2_GetActorLocation`) (* (`KismetMathLibrary.RandomUnitVector`) (`KismetMathLibrary.RandomIntegerInRange` -10 10)))))
  (set `self.EndLocation` (+ _output_get (`self.Offset`)))
  (bind (_direction _movetrack) (`Timeline|MoveT`)
    (:`Update`
      (`self.K2_SetActorLocation` (`KismetMathLibrary.VLerp` (`self.StartLocation`) (`self.EndLocation`) _movetrack)))
    (:`Finished`
      (`self.K2_DestroyActor`))))

(fn `UserConstructionScript`)