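; BP_DeadLava is a lava hazard that deals lethal-scale damage to BP_MainMen characters on contact.
; The Construction Script tiles an instanced static mesh into a square grid, with spacing from Size and scale from SizeInt, both relative to the actor transform.
; The mesh's overlap and hit events share one path that casts the other actor to BP_MainMen and applies the damage.
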(event `self.InstancedStaticMesh.OnComponentBeginOverlap`
  (params (OverlappedComponent :type "PrimitiveComponent Object Reference") (OtherActor :type "Actor Object Reference") (OtherComp :type "PrimitiveComponent Object Reference") (OtherBodyIndex :type Integer) (bFromSweep :type Boolean) (SweepResult :type "HitResult Structure (by ref)"))
  (bind _asbp_main_men (cast `/Game/Player/BP_MainMen` (stale `self.InstancedStaticMesh.OnComponentHit` OtherActor) :!label _label))
  (`GameplayStatics.ApplyDamage` _asbp_main_men 1000.0))

(event `self.InstancedStaticMesh.OnComponentHit`
  (params (HitComponent :type "PrimitiveComponent Object Reference") (OtherActor :type "Actor Object Reference") (OtherComp :type "PrimitiveComponent Object Reference") (NormalImpulse :type "Vector Structure") (Hit :type "HitResult Structure (by ref)"))
  (goto _label))

(fn `UserConstructionScript`
  (bind (_returnvalue_location _returnvalue_rotation _returnvalue_scale) (`KismetMathLibrary.BreakTransform` (`self.GetTransform`)))
  (bind (_size_x _size_y _size_z) (`KismetMathLibrary.BreakVector` (`self.Size`)))
  (for _index (range 11)
    (for _index_2 (range 11)
      (`InstancedStaticMeshComponent.AddInstance` (`self.InstancedStaticMesh`) (`KismetMathLibrary.MakeTransform` (+ _returnvalue_location (* (`self.Size`) (`KismetMathLibrary.MakeVector` (* _size_x _index_2) (* _size_y _index) _size_z))) _returnvalue_rotation (* _returnvalue_scale (`self.SizeInt`))) false))))