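; BP_Key is a spinning pickup that grants a player the end key.
; Tick rotates the Pivot component around yaw at RotationSpeed scaled by delta time.
; On overlap, the server alone follows the character to its controller and player state, sets HasEndKey on that player state, then destroys the key actor.
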(event `self.ReceiveTick`
  (params (DeltaSeconds :type "Float (single-precision)"))
  (bind _pivot (`self.Pivot`))
  (bind (_relativerotation_roll _relativerotation_pitch _relativerotation_yaw) (`KismetMathLibrary.BreakRotator` (`SceneComponent.RelativeRotation` _pivot)))
  (`SceneComponent.K2_SetRelativeRotation` _pivot (`KismetMathLibrary.MakeRotator` _relativerotation_roll _relativerotation_pitch (+ _relativerotation_yaw (* DeltaSeconds (`self.RotationSpeed`)))) false false))

(event `self.ReceiveActorBeginOverlap`
  (params (OtherActor :type "Actor Object Reference"))
  (`/Engine/EditorBlueprintResources/ActorMacros.Switch Has Authority`
    (:`Authority`
      (bind _asbp_my_character (cast `/Game/Blueprints/Player/BP_MyCharacter` OtherActor))
      (bind _asbp_my_player_controller (cast `/Game/Blueprints/Player/BP_MyPlayerController` (`Pawn.GetController` _asbp_my_character)))
      (bind _asbp_my_player_state (cast `/Game/Blueprints/Player/BP_MyPlayerState` (`Controller.PlayerState` _asbp_my_player_controller)))
      (set `/Game/Blueprints/Player/BP_MyPlayerState.HasEndKey` true _asbp_my_player_state)
      (`self.K2_DestroyActor`))))

(fn `UserConstructionScript`)