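; BP_MyDoor is a lockable swinging door whose open and close events set a target yaw angle.
; TryUnlockDoor checks the caller's player state for an end key, then unlocks RoomA and RoomB and opens the door.
; The Interact, lock-material and Tick rotation logic is disconnected, so those events do nothing in this Blueprint and TryUnlockDoor is only called from unwired nodes.
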(event `Set Locked Material`
  (params (Locked :type Boolean)))

(event `self.ReceiveBeginPlay`)

(event `self.OnDoorLock_BP`)

(event `self.OnDoorUnlock_BP`)

(event `self.ReceiveTick`
  (params (DeltaSeconds :type "Float (single-precision)")))

(event `self.OnDoorOpen_BP`
  (set `self.TargetDoorAngle` 90.0))

(event `self.OnDoorClose_BP`
  (set `self.TargetDoorAngle` 0.0))

(event `/Game/Blueprints/Interfaces/IInteractable.Interact`
  (params (Caller :type "Actor Object Reference")))

(fn `CanInteract`
  (params (Caller :type "Actor Object Reference"))
  (returns (ReturnValue :type Boolean))
  (return (not (`self.IsLocked`))))

(fn `TryUnlockDoor`
  (params (Caller :type "Actor Object Reference"))
  (bind _aspawn (cast `Pawn` Caller)
    (:`then`
      (bind _asbp_my_player_controller (cast `/Game/Blueprints/Player/BP_MyPlayerController` (`Pawn.GetController` _aspawn))
        (:`then`
          (bind _asbp_my_player_state (cast `/Game/Blueprints/Player/BP_MyPlayerState` (`Controller.PlayerState` _asbp_my_player_controller))
            (:`then`
              (if (`/Game/Blueprints/Player/BP_MyPlayerState.HasEndKey` _asbp_my_player_state)
                ;[1 1 1] Should be both valid with this door actor
                (`Room.Lock` (`self.RoomA`) false)
                (`Room.Lock` (`self.RoomB`) false)
                (`self.Open` true)
                (else
                  (`KismetSystemLibrary.PrintString` "UNLOCK: No key" true true (struct :`R` 1.0 :`G` 0.087707 :`A` 1.0) 5.0))))
            (:`CastFailed`
              (`KismetSystemLibrary.PrintString` "UNLOCK: No Player state" true true (struct :`R` 1.0 :`G` 0.087707 :`A` 1.0) 5.0))))
        (:`CastFailed`
          (`KismetSystemLibrary.PrintString` "UNLOCK: No Player Controller" true true (struct :`R` 1.0 :`G` 0.087707 :`A` 1.0) 5.0))))
    (:`CastFailed`
      (`KismetSystemLibrary.PrintString` "UNLOCK: Caller is not Pawn" true true (struct :`R` 1.0 :`G` 0.087707 :`A` 1.0) 5.0))))

(fn `UserConstructionScript`)