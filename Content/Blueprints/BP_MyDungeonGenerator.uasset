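; BP_MyDungeonGenerator procedurally builds a lock-and-key dungeon on BeginPlay, switching player 0 to spectate during generation and restarting them afterward.
; Room selection starts at StartRoom, adds random non-repeating rooms, and inserts KeyRoom and EndRoom past count thresholds, both required for validity.
; Connections between two rooms get doors, others walls.
; Initialization locks the end room and assigns the key to KeyRoom's custom data if reachable from start through unlocked rooms.
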(event `self.ReceiveBeginPlay`
  (`self.Generate`))

(event `self.OnPreGeneration`
  (`parent.OnPreGeneration`) ; Calls the C++ implementation.\nDefault implementation dispatch OnPreGeneration event.\nYou can put it later in the function if you want.
  (`KismetSystemLibrary.PrintString` "Dungeon Begin Generation..." true true (struct :`G` 0.66 :`B` 1.0 :`A` 1.0) 20.0)
  (bind _asbp_my_player_controller (cast `/Game/Blueprints/Player/BP_MyPlayerController` (`GameplayStatics.GetPlayerController` 0)))
  (`/Game/Blueprints/Player/BP_MyPlayerController.Server_Spectate` _asbp_my_player_controller))

(event `self.OnPostGeneration`
  (`parent.OnPostGeneration`) ; Calls the C++ implementation.\nDefault implementation dispatch OnPostGeneration event.\nYou can put it later in the function if you want.
  (`KismetSystemLibrary.PrintString` "Dungeon Generated!" true true (struct :`G` 0.66 :`B` 1.0 :`A` 1.0) 20.0)
  (bind _asbp_my_player_controller (cast `/Game/Blueprints/Player/BP_MyPlayerController` (`GameplayStatics.GetPlayerController` 0)))
  (`/Game/Blueprints/Player/BP_MyPlayerController.Server_RestartPlayer` _asbp_my_player_controller))

(fn `ChooseDoor`
  (params (CurrentRoom :type "RoomData Object Reference") (NextRoom :type "RoomData Object Reference") (DoorType :type "DoorType Object Reference"))
  (returns (ReturnValue :type "Door Class Reference"))
  (if (and (`KismetSystemLibrary.IsValid` CurrentRoom) (`KismetSystemLibrary.IsValid` NextRoom))
    (return "/Game/Blueprints/BP_MyDoor.BP_MyDoor_C")
    (else
      (return "/Game/Blueprints/BP_Wall.BP_Wall_C"))))

(fn `ChooseFirstRoomData`
  (returns (ReturnValue :type "RoomData Object Reference"))
  (return (`self.StartRoom`)))

(fn `ChooseNextRoomData`
  (params (CurrentRoom :type "RoomData Object Reference") (DoorData :type "DoorDef Structure (by ref)"))
  (returns (ReturnValue :type "RoomData Object Reference"))
  (bind _graph (`self.Graph`))
  (if (and (not (`DungeonGraph.HasAlreadyRoomData` _graph (`self.KeyRoom`))) (> (`DungeonGraph.Count` _graph) (`self.RoomBeforeKey`)))
    (return (`self.KeyRoom`))
    (elif (> (`DungeonGraph.Count` (`self.Graph`)) (+ (`self.RoomBeforeKey`) (`self.AdditionalRooms`)))
      (return (`self.EndRoom`))
      (else
        (bind _random (`self.GetRandomRoomWithExclusion` (`self.RandomRooms`) (`|MakeSet` CurrentRoom)))
        (return _random)))))

(fn `ContinueToAddRoom`
  (returns (ReturnValue :type Boolean))
  (return (not (`DungeonGraph.HasAlreadyRoomData` (`self.Graph`) (`self.EndRoom`)))))

(fn `GetRandomRoomWithExclusion`
  (params (RoomData :type "Array of RoomData Object Reference") (ExclusionList :type "Set of RoomData Object Reference"))
  (returns (Random :type "RoomData Object Reference"))
  (locals (Loop :type Boolean :default true) (ChosenRoom :type "RoomData Object Reference"))
  (while (`local.Loop`)
    (bind _returnvalue (`self.GetRandomRoomData` (`local.RoomData`)))
    (if (not (`BlueprintSetLibrary.Set_Contains` (`local.ExclusionList`) _returnvalue))
      (set `local.ChosenRoom` _returnvalue)
      (set `local.Loop` false)))
  (return (`local.ChosenRoom`)))

(fn `InitializeDungeon`
  (params (Rooms :type "DungeonGraph Object Reference"))
  (locals (EndRoomInstance :type "Room Object Reference") (KeyRoomInstance :type "Room Object Reference") (StartRoomInstance :type "Room Object Reference"))
  (`|ExecutionSequence`
    (:`then_0`
      ;[1 1 1] Lock End Room
      (bind _returnvalue (`DungeonGraph.GetFirstRoomFromData` Rooms (`self.EndRoom`))) ; I know there is only one end room
      (bind _output_get (set `local.EndRoomInstance` _returnvalue))
      (`/Engine/EditorBlueprintResources/StandardMacros.IsValid` _output_get
        (:`Is Valid`
          (`Room.Lock` _returnvalue true))
        (:`Is Not Valid`
          (`KismetSystemLibrary.PrintString` "ERROR: No end room in generated dungeon" true true (struct :`R` 1.0 :`A` 1.0) 10.0))))
    (:`then_1`
      ;[1 1 1] Place Key in Dungeon if Valid Path From Start Room
      (bind _returnvalue_2 (`DungeonGraph.GetFirstRoomFromData` Rooms (`self.KeyRoom`))) ; I know there is only one key room
      (bind _output_get_2 (set `local.KeyRoomInstance` _returnvalue_2))
      (`/Engine/EditorBlueprintResources/StandardMacros.IsValid` _output_get_2
        (:`Is Valid`
          (bind _returnvalue_3 (`DungeonGraph.GetFirstRoomFromData` (`self.Graph`) (`self.StartRoom`))) ; I know there is only one start room
          (bind _output_get_3 (set `local.StartRoomInstance` _returnvalue_3))
          (`/Engine/EditorBlueprintResources/StandardMacros.IsValid` _output_get_3
            (:`Is Valid`
              (bind _returnvalue_4 (`DungeonGraph.HasValidPath` (`self.Graph`) (`local.StartRoomInstance`) (`local.KeyRoomInstance`) false))
              (if _returnvalue_4
                (bind _data (`Room.GetCustomData_BP` (`local.KeyRoomInstance`) "/Game/Blueprints/BP_KeyCustomData.BP_KeyCustomData_C")
                  (:`True`
                    (set `/Game/Blueprints/BP_KeyCustomData.KeyToSpawn` "/Game/Blueprints/BP_Key.BP_Key_C" _data))
                  (:`False`
                    (`KismetSystemLibrary.PrintString` "ERROR: Key room has no Key Custom Data" true true (struct :`R` 1.0 :`A` 1.0) 10.0)))))
            (:`Is Not Valid`
              (`KismetSystemLibrary.PrintString` "ERROR: No start room in generated dungeon" true true (struct :`R` 1.0 :`A` 1.0) 10.0))))
        (:`Is Not Valid`
          (`KismetSystemLibrary.PrintString` "ERROR: No key room in generated dungeon" true true (struct :`R` 1.0 :`A` 1.0) 10.0))))))

(fn `IsValidDungeon`
  (returns (ReturnValue :type Boolean))
  (bind _graph (`self.Graph`))
  (return (and (`DungeonGraph.HasAlreadyRoomData` _graph (`self.EndRoom`)) (`DungeonGraph.HasAlreadyRoomData` _graph (`self.KeyRoom`)))))

(fn `UserConstructionScript`)