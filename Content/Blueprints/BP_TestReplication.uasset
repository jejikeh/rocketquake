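; BP_TestReplication is an interactable test actor that cycles the material on its Cube and replicates the change to clients.
; Interact runs on the server, advancing the CurrentMaterial index with wraparound through MaterialList, then applies it via UpdateMaterial.
; Clients receive the index through OnRep_CurrentMaterial, which calls the same UpdateMaterial.
; CanInteract always returns true, so any caller can trigger it.
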(event `/Game/Blueprints/Interfaces/IInteractable.Interact`
  (params (Caller :type "Actor Object Reference"))
  ;[1 1 1] The interaction is called on the server, it will replicate the material index to clients
  (set `self.CurrentMaterial` (mod (+ (`self.CurrentMaterial`) 1) (`KismetArrayLibrary.Array_Length` (`self.MaterialList`)))) ; The client should never modify the replicated variable.\nThe server will take care of it and replicate it on clients.\nThen the clients can use it from the OnRep_XXX function.
  (`self.UpdateMaterial`))

(event `OnRep_CurrentMaterial`
  ;[1 1 1] Update the material on clients when the index is received from server
  (`self.UpdateMaterial`))

(event `UpdateMaterial`
  (`PrimitiveComponent.SetMaterial` (`self.Cube`) 0 (`|GetArrayItem` (`self.MaterialList`) (`self.CurrentMaterial`))))

(fn `CanInteract`
  (params (Caller :type "Actor Object Reference"))
  (returns (ReturnValue :type Boolean))
  (return true))

(fn `UserConstructionScript`)