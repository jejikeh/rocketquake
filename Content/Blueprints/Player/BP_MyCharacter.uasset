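; BP_MyCharacter is the player character Blueprint, handling movement, camera look and interaction with world objects.
; Enhanced Input actions drive movement relative to control rotation and apply yaw and pitch to the camera.
; The interact input sends a server RPC, so interaction logic runs with server authority.
; The server runs a short Visibility line trace from the eye viewpoint and calls Interact through the IInteractable interface on a valid hit.
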(event `EnhancedInput|/Game/Blueprints/Player/Inputs/Input_Interact`
  (params (ActionValue :type Boolean) (ElapsedSeconds :type "Float (double-precision)") (TriggeredSeconds :type "Float (double-precision)") (InputAction :type "InputAction Object Reference" :default "/Game/Blueprints/Player/Inputs/Input_Interact.Input_Interact"))
  ;[1 1 1] The client player press the input to interact.
  ; We send an RPC to the server to make the interaction logic there.
  (:`Triggered`
    (`self.Server_Interact`)))

(event `EnhancedInput|/Game/Blueprints/Player/Inputs/Input_Move`
  (params (ActionValue :type "Vector2D Structure") (ElapsedSeconds :type "Float (double-precision)") (TriggeredSeconds :type "Float (double-precision)") (InputAction :type "InputAction Object Reference" :default "/Game/Blueprints/Player/Inputs/Input_Move.Input_Move"))
  (bind (_returnvalue_roll _returnvalue_pitch _returnvalue_yaw) (`KismetMathLibrary.BreakRotator` (`self.GetControlRotation`)))
  (bind (_returnvalue_roll_2 _returnvalue_pitch_2 _returnvalue_yaw_2) (`KismetMathLibrary.BreakRotator` (`self.GetControlRotation`)))
  ;[1 1 1] Handling movement inputs
  (:`Triggered`
    (`self.AddMovementInput` (`KismetMathLibrary.GetRightVector` (`KismetMathLibrary.MakeRotator` _returnvalue_roll_2 0.0 _returnvalue_yaw_2)) ActionValue_X)
    (`self.AddMovementInput` (`KismetMathLibrary.GetForwardVector` (`KismetMathLibrary.MakeRotator` 0.0 0.0 _returnvalue_yaw)) ActionValue_Y)))

(event `Server_Interact`
  ;[1 1 1] This function is executed on server side.
  ; We get the interactable if any and call the Interact interface on it.
  (bind _interactable (`self.GetInteractable`)) ; Custom function
  (`/Engine/EditorBlueprintResources/StandardMacros.IsValid` (`KismetSystemLibrary.Conv_InterfaceToObject` _interactable)
    (:`Is Valid`
      (`/Game/Blueprints/Interfaces/IInteractable.Interact` _interactable self) ; Good practice: use an interface
    )))

(event `EnhancedInput|/Game/Blueprints/Player/Inputs/Input_Camera`
  (params (ActionValue :type "Vector2D Structure") (ElapsedSeconds :type "Float (double-precision)") (TriggeredSeconds :type "Float (double-precision)") (InputAction :type "InputAction Object Reference" :default "/Game/Blueprints/Player/Inputs/Input_Camera.Input_Camera"))
  ;[1 1 1] Handling camera inputs
  (:`Triggered`
    (`self.AddControllerYawInput` ActionValue_X)
    (`self.AddControllerPitchInput` ActionValue_Y)))

(fn `GetInteractable`
  (returns (Interactable :type "/Game/Blueprints/Interfaces/IInteractable Interface"))
  (bind (_outlocation _outrotation) (`self.GetActorEyesViewPoint`))
  (bind (_outhit _returnvalue) (`KismetSystemLibrary.LineTraceSingle` :`Start` _outlocation :`End` (+ _outlocation (* (`KismetMathLibrary.GetForwardVector` _outrotation) 200.0)) :`TraceChannel` "TraceTypeQuery1" :`DrawTime` 20.0))
  (if _returnvalue
    (return (cast `/Game/Blueprints/Interfaces/IInteractable` (`.HitActor` (`GameplayStatics.BreakHitResult` _outhit)) :!pure true))
    (else
      (return null))))

(fn `UserConstructionScript`)