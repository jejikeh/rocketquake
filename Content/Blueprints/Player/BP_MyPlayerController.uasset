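; Player controller for a dungeon generator game, handling input mapping, dungeon generation, spectating and HUD refresh.
; Input triggers the first DungeonGenerator or server-side spectating, and a debug key destroys all generators.
; Server_RestartPlayer respawns the player at a random horizontal offset around the "Dungeon Start" player start.
; Pawn changes refresh the HUD and destroy the previous BP_MyCharacter; a delayed BeginPlay refresh works around HUD input display.
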(event Custom|GenerateDungeon
  (bind _outactors (Actor|GetAllActorsOfClass "/Script/ProceduralDungeon.DungeonGenerator"))
  (if (Utilities|Array|IsNotEmpty _outactors)
    (PCG|Generate (Utilities|Array|Get(acopy) _outactors))))

(event Custom|Client_OnStateChanged
  ;[1 1 1] Spectating
  (CallFunction|UpdateHUD))

(event Custom|Server_Spectate
  ;[1 1 1] Spectating
  (Class|DungeonBlueprintLibrary|Spectate 0 false)
  (CallFunction|ClientonStateChanged))

(event Custom|Server_RestartPlayer
  (bind _returnvalue (Game|GetGameMode))
  (bind _self self)
  (bind _returnvalue_2 (Class|GameModeBase|FindPlayerStart _returnvalue _self "Dungeon Start"))
  (bind _returnvalue_3 (Transformation|GetActorTransform _returnvalue_2))
  ;[1 1 1] Teleport Player to Dungeon Start
  (Class|GameModeBase|RestartPlayeratTransform _returnvalue _self (Math|Transform|MakeTransform (+ (.location _returnvalue_3) (* (Class|KismetMathLibrary|VectorNormal2D (Math|Random|RandomUnitVector) 0.0001) 2e+02)) (.rotation _returnvalue_3) (.scale _returnvalue_3))))

(event Custom|OnPawnChanged
  (params (OldPawn :type Pawn%20Object%20Reference) (NewPawn :type Pawn%20Object%20Reference))
  (Development|PrintString "On Pawn Changed" true true "(R=1.000000,G=0.000000,B=0.662548,A=1.000000)" 2e+01)
  (CallFunction|UpdateHUD)
  (bind _asbp_my_character (Utilities|Casting|CastToBP_MyCharacter OldPawn))
  (Actor|DestroyActor _asbp_my_character)
  (Development|PrintString "Previous pawn destroyed" true true "(R=1.000000,G=0.990346,B=0.000000,A=1.000000)" 2e+01))

(event Input|EnhancedActionEvents|EnhancedInputActionInput_Generate
  (params (ActionValue :type Boolean) (ElapsedSeconds :type Float%20%28double-precision%29) (TriggeredSeconds :type Float%20%28double-precision%29) (InputAction :type Input%20Action%20Object%20Reference :default "/Game/Blueprints/Player/Inputs/Input_Generate.Input_Generate"))
  (:Triggered
    (CallFunction|GenerateDungeon)))

(event Input|EnhancedActionEvents|EnhancedInputActionInput_Spectate
  (params (ActionValue :type Boolean) (ElapsedSeconds :type Float%20%28double-precision%29) (TriggeredSeconds :type Float%20%28double-precision%29) (InputAction :type Input%20Action%20Object%20Reference :default "/Game/Blueprints/Player/Inputs/Input_Spectate.Input_Spectate"))
  (:Triggered
    (CallFunction|ServerSpectate)))

(event EventBeginPlay
  (bind _self self)
  (bind _returnvalue (PlayerController|LocalPlayerSubsystems|GetEnhancedInputLocalPlayerSubsystem _self))
  (Utilities|IsValid _returnvalue
    (:Is%20Valid
      (Input|AddMappingContext _returnvalue "/Game/Blueprints/Player/Inputs/InputContext_Default.InputContext_Default" 0 "(bIgnoreAllPressedKeysUntilRelease=True,bForceImmediately=False)")
      (Pawn|BindEventtoOnPossessedPawnChanged (delegate Custom|OnPawnChanged))
      (Utilities|FlowControl|Delay 0.5) ; Hack to display correctly inputs in HUD
      (CallFunction|UpdateHUD))))

(event Input|KeyboardEvents|DebugKeyDelete
  (params (Key :type Key%20Structure) (ActionValue :type Input%20Action%20Value%20Structure))
  ;[0 0 0] Just a debug key to test Dungeon Generator destroying
  (:Pressed
    (bind _outactors (Actor|GetAllActorsOfClass "/Script/ProceduralDungeon.DungeonGenerator"))
    (for _array_element _outactors
      (Actor|DestroyActor _array_element))))

(fn ConstructionScript)

(fn UpdateHUD
  (bind _asbp_player_hud (Utilities|Casting|CastToBP_PlayerHUD (HUD|GetHUD)))
  (Default|OnPawnChanged _asbp_player_hud self))