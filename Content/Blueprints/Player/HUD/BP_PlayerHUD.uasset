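; Player HUD Blueprint that shows the W_MainScreen widget as a spectator HUD and links it to the player's controller.
; On OnPawnChanged it casts the passed controller to BP_MyPlayerController, creates and adds the widget to the viewport only if none exists, then hands it that controller.
; Debug strings report a successful update or a failed cast.
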(event `OnPawnChanged`
  (params (Controller :type "Controller Object Reference"))
  (bind _asbp_my_player_controller (cast `/Game/Blueprints/Player/BP_MyPlayerController` Controller)
    (:`then`
      (`|ExecutionSequence`
        (:`then_0`
          (`/Engine/EditorBlueprintResources/StandardMacros.IsValid` (`self.SpectatorHUD`)
            (:`Is Not Valid`
              (bind _returnvalue (`|CreateWidget` "/Game/Blueprints/Player/HUD/W_MainScreen.W_MainScreen_C"))
              (bind _output_get (set `self.SpectatorHUD` _returnvalue))
              (`UserWidget.AddToViewport` _output_get 0))))
        (:`then_1`
          (`/Game/Blueprints/Player/HUD/W_MainScreen.Set Controller` (`self.SpectatorHUD`) _asbp_my_player_controller)
          (`KismetSystemLibrary.PrintString` "Updated Success!" true true (struct :`R` 1.0 :`G` 0.490895 :`A` 1.0) 20.0))))
    (:`CastFailed`
      (`KismetSystemLibrary.PrintString` "No Controller!" true true (struct :`R` 1.0 :`G` 0.006082 :`A` 1.0) 20.0))))

(fn `UserConstructionScript`)