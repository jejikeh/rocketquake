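; BP_FriendList is a menu actor that hosts the Steam friends list widget and toggles its visibility.
; On BeginPlay it binds the widget's close click to hide the actor through Show.
; Show turns off the stored lobby player platform's friends list whether showing or hiding, but assigns that reference to itself rather than to FromLobbyPlayerPlatform when showing.
; Hiding clears the reference and fires OnHideVisibility.
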(event `self.ReceiveBeginPlay`
  (bind _aswbp_steam_friends_list (cast `/Game/UI/WBP_SteamFriendsList` (`WidgetComponent.GetWidget` (`self.Widget`))))
  (add `/Game/UI/WBP_SteamFriendsList.OnCloseClicked` _aswbp_steam_friends_list (delegate `HandleClick`)))

(event `HandleClick`
  (`self.Show` false))

(fn `Show`
  (params (Show :type Boolean) (FromLobbyPlayerPlatform :type "/Game/Menu/BP_LobbyPlayerPlatform Object Reference"))
  (bind _lastlobbyplayerplatform (`self.LastLobbyPlayerPlatform`))
  (bind _lastlobbyplayerplatform_2 (`self.LastLobbyPlayerPlatform`))
  (if Show
    (`self.SetActorHiddenInGame` false)
    (`/Engine/EditorBlueprintResources/StandardMacros.IsValid` _lastlobbyplayerplatform_2
      (:`Is Valid`
        (`/Game/Menu/BP_LobbyPlayerPlatform.ShowFriendsList` _lastlobbyplayerplatform_2 false))
      (:`Is Not Valid`
        _))
    (set `self.LastLobbyPlayerPlatform` (`self.LastLobbyPlayerPlatform`))
    (else
      (`self.SetActorHiddenInGame` true)
      (`/Engine/EditorBlueprintResources/StandardMacros.IsValid` _lastlobbyplayerplatform
        (:`Is Valid`
          (`/Game/Menu/BP_LobbyPlayerPlatform.ShowFriendsList` _lastlobbyplayerplatform false))
        (:`Is Not Valid`
          _))
      (set `self.LastLobbyPlayerPlatform` null)
      (`self.OnHideVisibility`))))

(fn `UserConstructionScript`)