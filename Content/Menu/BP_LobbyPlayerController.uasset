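; Lobby player controller that reports this player's info and ready state to the menu game mode.
; On BeginPlay, the local controller calls ServerSetName; name-set, ready-toggle and delayed retry events all route through BP_MenuGameModeBase's UpdatePlayerInfo.
; Ready toggling flips the flag in the player's lobby info struct before updating.
; StartMatch shows the main menu's loading screen; the lobby widget creation in SetupUp is disconnected.
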(event `self.ReceiveBeginPlay`
  (`self.SetupUp`))

(event `TryAgainUpdate`
  (`KismetSystemLibrary.Delay` 0.2)
  (bind _asbp_menu_game_mode_base (cast `/Game/Menu/BP_MenuGameModeBase` (`GameplayStatics.GetGameMode`)))
  (`/Game/Menu/BP_MenuGameModeBase.UpdatePlayerInfo` _asbp_menu_game_mode_base self))

(event `Server_SetName`
  (bind _asbp_menu_game_mode_base (cast `/Game/Menu/BP_MenuGameModeBase` (`GameplayStatics.GetGameMode`)))
  (`/Game/Menu/BP_MenuGameModeBase.UpdatePlayerInfo` _asbp_menu_game_mode_base self))

(event `ServerToggleReady`
  (bind _playerlobbyinfopc (`self.PlayerLobbyInfoPC`))
  (setmembers `/Game/Menu/BP_PlayerLobbyInfo` :`StructRef` _playerlobbyinfopc :`Ready` (not (`.Ready_8_6A06C164CE42B7A1C662508337EE9E6C` (break `/Game/Menu/BP_PlayerLobbyInfo` _playerlobbyinfopc))))
  (bind _asbp_menu_game_mode_base (cast `/Game/Menu/BP_MenuGameModeBase` (`GameplayStatics.GetGameMode`)))
  (`/Game/Menu/BP_MenuGameModeBase.UpdatePlayerInfo` _asbp_menu_game_mode_base self))

(event `StartMatch`
  (bind _aswbp_main_menu (cast `/Game/UI/WBP_MainMenu` (`self.GetMenuWidget`)))
  (`/Game/UI/WBP_MainMenu.ShowLoadingScreen` _aswbp_main_menu))

(fn `SetupUp`
  (if (`self.IsLocalPlayerController`)
    (`self.Server_SetName`)))

(fn `UserConstructionScript`)