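; Lobby platform actor that displays one player's menu character, or a button to open the friend list while the slot is empty.
; On the server, it finds the shared BP_FriendList, links the button widget to itself and restores the button when the list hides.
; Opening moves that list to this platform.
; SpawnCharacter replaces the character, hiding the button and any list at the button's location; Clear reverses this.
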(event `self.ReceiveBeginPlay`
  (`self.SetUpServer`)
  (if (`KismetSystemLibrary.IsServer`)
    (add `/Game/Menu/BP_FriendList.OnHideVisibility` (`self.FriendList`) (delegate `ShowOnHide`))))

(event `ShowOnHide`
  (`self.ShowFriendsList` false))

(event `SpawnCharacter`
  (params (PC :type "PlayerController Object Reference"))
  (bind _currentcharacter (`self.CurrentCharacter`))
  (set `self.PC` PC)
  (`/Engine/EditorBlueprintResources/StandardMacros.IsValid` _currentcharacter
    (:`Is Valid`
      (`self.K2_DestroyActor` _currentcharacter))
    (:`Is Not Valid`
      _))
  (bind _returnvalue (`|SpawnActorFromClass` "/Game/Player/BP_MainMenMenu.BP_MainMenMenu_C" (`SceneComponent.K2_GetComponentToWorld` (`self.PlayerSpawnTransform`)) "Undefined" "MultiplyWithRoot" null null))
  (set `self.CurrentCharacter` _returnvalue)
  (`SceneComponent.SetVisibility` (`self.OpenFriendList`) false false)
  (if (== (`self.K2_GetActorLocation` (`self.FriendList`)) (`SceneComponent.K2_GetComponentLocation` (`self.OpenFriendList`)) :`ErrorTolerance` 1.0)
    (`/Game/Menu/BP_FriendList.Show` (`self.FriendList`) false null)))

(event `Clear`
  (bind _currentcharacter (`self.CurrentCharacter`))
  (set `self.PC` null)
  (`/Engine/EditorBlueprintResources/StandardMacros.IsValid` _currentcharacter
    (:`Is Valid`
      (`self.K2_DestroyActor` _currentcharacter))
    (:`Is Not Valid`
      _))
  (set `self.CurrentCharacter` null)
  (`SceneComponent.SetVisibility` (`self.OpenFriendList`) true false))

(fn `SetUpServer`
  (if (`KismetSystemLibrary.IsServer`)
    (bind _returnvalue (`GameplayStatics.GetActorOfClass` "/Game/Menu/BP_FriendList.BP_FriendList_C"))
    (set `self.FriendList` _returnvalue)
    (bind _aswbp_open_friend_list_button (cast `/Game/UI/WBP_OpenFriendListButton` (`WidgetComponent.GetWidget` (`self.OpenFriendList`))))
    (set `/Game/UI/WBP_OpenFriendListButton.LobbyPlatformRef` self _aswbp_open_friend_list_button)
    (`SceneComponent.SetVisibility` (`self.OpenFriendList`) true false)))

(fn `ShowFriendsList`
  (params (Show :type Boolean))
  (bind _friendlist (`self.FriendList`))
  (bind _returnvalue (`WidgetComponent.GetWidget` (`self.OpenFriendList`)))
  (if Show
    (`Widget.SetVisibility` _returnvalue "Collapsed")
    (`self.K2_SetActorLocation` _friendlist (`SceneComponent.K2_GetComponentLocation` (`self.FriendListLocation`)) false false)
    (`/Game/Menu/BP_FriendList.Show` _friendlist true self)
    (else
      (`Widget.SetVisibility` _returnvalue "Visible"))))

(fn `UserConstructionScript`)