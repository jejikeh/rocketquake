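; Game mode for the menu lobby that seats joining players on tagged BP_LobbyPlayerPlatform actors and hosts the match.
; Platforms are gathered by index tag at BeginPlay; logins and logouts wait on a polling macro, then spawn or clear platform characters.
; UpdatePlayerInfo pushes name and ready state to characters, then CheckReadyCount sets the host menu's all-ready flag.
; HostMatch server-travels to L_Showcase and notifies each lobby controller; KickPC removes players.
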(event `self.ReceiveBeginPlay`
  (`self.SetUpPlatforms`)
  (`WidgetBlueprintLibrary.SetInputMode_UIOnlyEx` (`GameplayStatics.GetPlayerController` 0) null))

(event `self.K2_PostLogin`
  (params (NewPlayer :type "PlayerController Object Reference"))
  (`KismetArrayLibrary.Array_Add` (`self.PCs`) NewPlayer)
  (`self.IsPlatfrormSetupIsDone` :!label _label
    (:`true`
      (`self.UpdatePlayersOnPlatforms`))))

(event `self.K2_OnLogout`
  (params (ExitingController :type "Controller Object Reference"))
  (bind _asplayer_controller (cast `PlayerController` ExitingController))
  (`KismetArrayLibrary.Array_RemoveItem` (`self.PCs`) _asplayer_controller)
  (goto _label))

(event `HostMatch`
  (`AdvancedSessionsLibrary.ServerTravel` "L_Showcase")
  (for _array_element (`self.PCs`)
    (bind _asbp_lobby_player_controller (cast `/Game/Menu/BP_LobbyPlayerController` _array_element))
    (`/Game/Menu/BP_LobbyPlayerController.StartMatch` _asbp_lobby_player_controller)))

(fn `CheckReadyCount`
  (locals (ReadyCount :type Boolean :default true))
  (set `local.ReadyCount` true)
  (for _array_element (`self.PCs`)
    (bind _asbp_lobby_player_controller (cast `/Game/Menu/BP_LobbyPlayerController` _array_element))
    (bind (_playerlobbyinfopc_pc _playerlobbyinfopc_playername _playerlobbyinfopc_ready) (break `/Game/Menu/BP_PlayerLobbyInfo` (`/Game/Menu/BP_LobbyPlayerController.PlayerLobbyInfoPC` _asbp_lobby_player_controller)))
    (if (not _playerlobbyinfopc_ready)
      (set `local.ReadyCount` false)))
  (bind _asbp_lobby_player_controller_2 (cast `/Game/Menu/BP_LobbyPlayerController` (`GameplayStatics.GetPlayerController` 0)))
  (bind _returnvalue (`MenuPlayerController.GetMenuWidget` _asbp_lobby_player_controller_2))
  (`/Engine/EditorBlueprintResources/StandardMacros.IsValid` _returnvalue
    (:`Is Valid`
      (bind _aswbp_main_menu (cast `/Game/UI/WBP_MainMenu` _returnvalue))
      (set `/Game/UI/WBP_MainMenu.EnoughPlayersReady` (`local.ReadyCount`) _aswbp_main_menu))
    (:`Is Not Valid`
      (`KismetSystemLibrary.PrintString` "Hello"))))

(fn `KickPC`
  (params (PlayerToKick :type "PlayerController Object Reference"))
  (`AdvancedSessionsLibrary.KickPlayer` PlayerToKick))

(fn `SetUpPlatforms`
  (bind _outactors (`GameplayStatics.GetAllActorsOfClass` "/Game/Menu/BP_LobbyPlayerPlatform.BP_LobbyPlayerPlatform_C"))
  (for _index (range (+ (`KismetArrayLibrary.Array_LastIndex` _outactors) 1))
    (bind _outactors_2 (`GameplayStatics.GetAllActorsOfClassWithTag` "/Game/Menu/BP_LobbyPlayerPlatform.BP_LobbyPlayerPlatform_C" (`KismetStringLibrary.Conv_StringToName` (`KismetStringLibrary.Conv_IntToString` _index))))
    (`KismetArrayLibrary.Array_Add` (`self.PlayerPlatforms`) (`|GetArrayItem` _outactors_2)))
  (set `self.PlatformSetup` true))

(fn `UpdatePlayerInfo`
  (params (ReqPC :type "PlayerController Object Reference"))
  (bind _reqpc (`local.ReqPC`))
  (for _array_element (`self.PlayerPlatforms`)
    (if (== (`/Game/Menu/BP_LobbyPlayerPlatform.PC` _array_element) ReqPC)
      (bind _asbp_main_men_menu (cast `/Game/Player/BP_MainMenMenu` (`/Game/Menu/BP_LobbyPlayerPlatform.CurrentCharacter` _array_element)))
      (bind _asbp_lobby_player_controller (cast `/Game/Menu/BP_LobbyPlayerController` (`local.ReqPC`)))
      (`/Game/Player/BP_MainMenMenu.UpdateLobbyInfo` _asbp_main_men_menu (make `/Game/Menu/BP_PlayerLobbyInfo` (`local.ReqPC`) (`KismetTextLibrary.Conv_StringToText` (`AdvancedSessionsLibrary.GetPlayerName` _reqpc)) (`.Ready_8_6A06C164CE42B7A1C662508337EE9E6C` (break `/Game/Menu/BP_PlayerLobbyInfo` (`/Game/Menu/BP_LobbyPlayerController.PlayerLobbyInfoPC` _asbp_lobby_player_controller))) (`Controller.PlayerState` _reqpc)))
      (`self.CheckReadyCount`)
      (return)))
  (bind _asbp_lobby_player_controller_2 (cast `/Game/Menu/BP_LobbyPlayerController` (`local.ReqPC`)))
  (`/Game/Menu/BP_LobbyPlayerController.TryAgainUpdate` _asbp_lobby_player_controller_2))

(fn `UpdatePlayersOnPlatforms`
  (locals (PlayerAlreadeAdded :type Boolean))
  (for _array_element (`self.PCs`)
    (`/Engine/EditorBlueprintResources/StandardMacros.IsValid` _array_element
      (:`Is Valid`
        (set `local.PlayerAlreadeAdded` false)
        (for _array_element_2 (`self.PlayerPlatforms`)
          (if (== (`/Game/Menu/BP_LobbyPlayerPlatform.PC` _array_element_2) _array_element)
            (set `local.PlayerAlreadeAdded` true)
            (break)))
        (if (not (`local.PlayerAlreadeAdded`))
          (for _array_element_3 (`self.PlayerPlatforms`)
            (`/Engine/EditorBlueprintResources/StandardMacros.IsValid` (`/Game/Menu/BP_LobbyPlayerPlatform.PC` _array_element_3)
              (:`Is Not Valid`
                (`/Game/Menu/BP_LobbyPlayerPlatform.SpawnCharacter` _array_element_3 _array_element)
                (break))))))))
  (for _array_element_4 (`self.PlayerPlatforms`)
    (if (not (`KismetArrayLibrary.Array_Contains` (`self.PCs`) (`/Game/Menu/BP_LobbyPlayerPlatform.PC` _array_element_4)))
      (`/Game/Menu/BP_LobbyPlayerPlatform.Clear` _array_element_4))))

(fn `UserConstructionScript`)