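; BP_MainMen is a player character Blueprint that sets game-only input on BeginPlay.
; Each Tick, on the authority or locally controlled instance, it stores the camera's world rotation and a pitch taken from base aim locally or the camera otherwise.
; Taking damage spawns a BP_DamagePoints actor at the character's transform, passing it the damage amount.
; The Niagara skeletal mesh event is an empty stub, with its override call left disconnected.
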(event `self.ReceiveBeginPlay`
  (`WidgetBlueprintLibrary.SetInputMode_GameOnly` (`GameplayStatics.GetPlayerController` 0)))

(event `self.ReceiveTick`
  (params (DeltaSeconds :type "Float (single-precision)"))
  (`self.GetControlRotation_Rep`))

(event `SetNiagaraSkeletalMesh_1`
  (params (NiagaraComponent :type "NiagaraComponent Object Reference")))

(event `self.ReceiveAnyDamage`
  (params (Damage :type "Float (single-precision)") (DamageType :type "DamageType Object Reference") (InstigatedBy :type "Controller Object Reference") (DamageCauser :type "Actor Object Reference"))
  (`|SpawnActorFromClass` "/Game/Blueprints/BP_DamagePoints.BP_DamagePoints_C" (`self.GetTransform`) "Undefined" "MultiplyWithRoot" null Damage null))

(fn `GetControlRotation_Rep`
  (bind (_returnvalue_roll _returnvalue_pitch) (`KismetMathLibrary.BreakRotator` (`self.GetBaseAimRotation`)))
  (bind _cameracomponent (`self.CameraComponent`))
  (bind (_returnvalue_roll_2 _returnvalue_pitch_2) (`KismetMathLibrary.BreakRotator` (`SceneComponent.K2_GetComponentRotation` _cameracomponent)))
  (if (or (`self.HasAuthority`) (`self.IsLocallyControlled`))
    (set `self.ControlRotation` (`SceneComponent.K2_GetComponentRotation` _cameracomponent))
    (if (`self.IsLocallyControlled`)
      (set `self.ControlRotationPitch` _returnvalue_pitch)
      (else
        (set `self.ControlRotationPitch` _returnvalue_pitch_2)))))

(fn `UserConstructionScript`)