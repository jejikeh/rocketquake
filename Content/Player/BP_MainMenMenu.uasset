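; Player character Blueprint, apparently for the main menu or lobby, that shows a lobby user tag and spawns damage-point actors when hit.
; BeginPlay sets game-only input, and Tick stores camera rotation and aim pitch on the authority or locally controlled instance.
; OnRep_LobbyInfo pushes lobby info into the WBP_LobbyUserTag widget, retrying on a short timer until that widget is valid.
; The Niagara skeletal-mesh event is an empty stub.
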(event `self.ReceiveBeginPlay`
  (`WidgetBlueprintLibrary.SetInputMode_GameOnly` (`GameplayStatics.GetPlayerController` 0)))

(event `self.ReceiveTick`
  (params (DeltaSeconds :type "Float (single-precision)"))
  (`self.GetControlRotation_Rep`))

(event `SetNiagaraSkeletalMesh_1`
  (params (NiagaraComponent :type "NiagaraComponent Object Reference")))

(event `self.ReceiveAnyDamage`
  (params (Damage :type "Float (single-precision)") (DamageType :type "DamageType Object Reference") (InstigatedBy :type "Controller Object Reference") (DamageCauser :type "Actor Object Reference"))
  (`|SpawnActorFromClass` "/Game/Blueprints/BP_DamagePoints.BP_DamagePoints_C" (`self.GetTransform`) "Undefined" "MultiplyWithRoot" null Damage null))

(fn `GetControlRotation_Rep`
  (bind (_returnvalue_roll _returnvalue_pitch) (`KismetMathLibrary.BreakRotator` (`self.GetBaseAimRotation`)))
  (bind _cameracomponent (`self.CameraComponent`))
  (bind (_returnvalue_roll_2 _returnvalue_pitch_2) (`KismetMathLibrary.BreakRotator` (`SceneComponent.K2_GetComponentRotation` _cameracomponent)))
  (if (or (`self.HasAuthority`) (`self.IsLocallyControlled`))
    (set `self.ControlRotation` (`SceneComponent.K2_GetComponentRotation` _cameracomponent))
    (if (`self.IsLocallyControlled`)
      (set `self.ControlRotationPitch` _returnvalue_pitch)
      (else
        (set `self.ControlRotationPitch` _returnvalue_pitch_2)))))

(fn `OnRep_LobbyInfo`
  (bind _returnvalue (`WidgetComponent.GetWidget` (`self.LobbyWidget`)))
  (`/Engine/EditorBlueprintResources/StandardMacros.IsValid` _returnvalue
    (:`Is Valid`
      (bind _aswbp_lobby_user_tag (cast `/Game/Menu/WBP_LobbyUserTag` _returnvalue))
      (`/Game/Menu/WBP_LobbyUserTag.Update` _aswbp_lobby_user_tag (`self.LobbyInfo`))
      (`SceneComponent.SetVisibility` (`self.LobbyWidget`) true false))
    (:`Is Not Valid`
      (`KismetSystemLibrary.K2_SetTimer` null "OnRep_LobbyInfo" 0.1))))

(fn `UpdateLobbyInfo`
  (params (LobbyInfo :type "/Game/Menu/BP_PlayerLobbyInfo Structure"))
  (set `self.LobbyInfo` LobbyInfo))

(fn `UserConstructionScript`)